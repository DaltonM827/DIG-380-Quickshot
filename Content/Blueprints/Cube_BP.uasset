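; Cube actor that changes its material each time it is hit.
; Three layers of nested FlipFlops in the Hit event act as a binary counter, cycling through eight materials such as woods, metals, stone and bush.
; Unconnected leftover logic holds a wrapping hit counter with actor destruction, plus a timeline that would rotate the cube and move it between two positions.
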(event `self.ReceiveHit`
  (params (MyComp :type "PrimitiveComponent Object Reference") (Other :type "Actor Object Reference") (OtherComp :type "PrimitiveComponent Object Reference") (bSelfMoved :type Boolean) (HitLocation :type "Vector Structure") (HitNormal :type "Vector Structure") (NormalImpulse :type "Vector Structure") (Hit :type "HitResult Structure (by ref)"))
  (bind _cube (`self.Cube`))
  (`/Engine/EditorBlueprintResources/StandardMacros.FlipFlop`
    (:`A`
      (`/Engine/EditorBlueprintResources/StandardMacros.FlipFlop`
        (:`A`
          (`/Engine/EditorBlueprintResources/StandardMacros.FlipFlop`
            (:`A`
              (`PrimitiveComponent.SetMaterial` _cube 0 "/Game/StarterContent/Materials/M_Wood_Walnut.M_Wood_Walnut"))
            (:`B`
              (`PrimitiveComponent.SetMaterial` _cube 0 "/Game/StarterContent/Materials/M_Metal_Burnished_Steel.M_Metal_Burnished_Steel"))))
        (:`B`
          (`/Engine/EditorBlueprintResources/StandardMacros.FlipFlop`
            (:`A`
              (`PrimitiveComponent.SetMaterial` _cube 0 "/Game/StarterContent/Materials/M_Metal_Copper.M_Metal_Copper"))
            (:`B`
              (`PrimitiveComponent.SetMaterial` _cube 0 "/Game/StarterContent/Materials/M_Metal_Gold.M_Metal_Gold"))))))
    (:`B`
      (`/Engine/EditorBlueprintResources/StandardMacros.FlipFlop`
        (:`A`
          (`/Engine/EditorBlueprintResources/StandardMacros.FlipFlop`
            (:`A`
              (`PrimitiveComponent.SetMaterial` _cube 0 "/Game/FPWeapon/Materials/FirstPersonProjectileMaterial.FirstPersonProjectileMaterial"))
            (:`B`
              (`PrimitiveComponent.SetMaterial` _cube 0 "/Game/StarterContent/Props/Materials/M_Bush.M_Bush"))))
        (:`B`
          (`/Engine/EditorBlueprintResources/StandardMacros.FlipFlop`
            (:`A`
              (`PrimitiveComponent.SetMaterial` _cube 0 "/Game/StarterContent/Materials/M_Brick_Hewn_Stone.M_Brick_Hewn_Stone"))
            (:`B`
              (`PrimitiveComponent.SetMaterial` _cube 0 "/Game/StarterContent/Materials/M_Wood_Oak.M_Wood_Oak"))))))))

(event `self.ReceiveTick`
  (params (DeltaSeconds :type "Float (single-precision)")))

(fn `UserConstructionScript`)