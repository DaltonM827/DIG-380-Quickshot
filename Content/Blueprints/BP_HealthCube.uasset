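; BP_HealthCube is a Blueprint that loses a small fixed amount of health each time it is hit.
; On Hit, it lowers CurrentHealth, creates a new WBP_HealthCube widget, copies the value into its PresentHealth, adds it to the viewport and prints it.
; Each hit adds another widget rather than updating an existing one.
; A CurrentHealth-to-MaxHealth ratio is left unused, and Tick and the construction script are empty.
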(event `self.ReceiveHit`
  (params (MyComp :type "PrimitiveComponent Object Reference") (Other :type "Actor Object Reference") (OtherComp :type "PrimitiveComponent Object Reference") (bSelfMoved :type Boolean) (HitLocation :type "Vector Structure") (HitNormal :type "Vector Structure") (NormalImpulse :type "Vector Structure") (Hit :type "HitResult Structure (by ref)"))
  (set `self.CurrentHealth` (- (`self.CurrentHealth`) 0.1))
  (bind _returnvalue (`|CreateWidget` "/Game/Blueprints/UI/WBP_HealthCube.WBP_HealthCube_C"))
  (bind _output_get (set `/Game/Blueprints/UI/WBP_HealthCube.PresentHealth` (`self.CurrentHealth`) _returnvalue))
  (`UserWidget.AddToViewport` _returnvalue 0)
  (`KismetSystemLibrary.PrintString` (`KismetStringLibrary.Conv_DoubleToString` _output_get)))

(event `self.ReceiveTick`
  (params (DeltaSeconds :type "Float (single-precision)")))

(fn `UserConstructionScript`)