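; BP_PracticeDummy is a shootable target dummy that loses health when hit by a first-person projectile.
; Each projectile hit subtracts fixed damage, prints the remaining health and adds a new MainHUD widget, as BeginPlay also does.
; When health exactly equals zero, it increments its own KillCounter, enables physics on body, head and neck, then destroys itself after a short delay.
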(event `self.ReceiveHit`
  (params (MyComp :type "PrimitiveComponent Object Reference") (Other :type "Actor Object Reference") (OtherComp :type "PrimitiveComponent Object Reference") (bSelfMoved :type Boolean) (HitLocation :type "Vector Structure") (HitNormal :type "Vector Structure") (NormalImpulse :type "Vector Structure") (Hit :type "HitResult Structure (by ref)"))
  (cast `/Game/FirstPerson/Blueprints/BP_FirstPersonProjectile` Other)
  (if true
    (bind _returnvalue (`|CreateWidget` "/Game/Blueprints/UI/MainHUD.MainHUD_C"))
    (`UserWidget.AddToViewport` _returnvalue 0)
    (bind _output_get (set `self.CurrentDummyHealth` (- (`self.CurrentDummyHealth`) 10.0)))
    (`KismetSystemLibrary.PrintString` (`KismetStringLibrary.Conv_DoubleToString` _output_get))
    (if (== _output_get 0.0)
      (set `self.KillCounter` (+ (`self.KillCounter`) 1))
      (`PrimitiveComponent.SetSimulatePhysics` (`self.Body`) true)
      (`PrimitiveComponent.SetSimulatePhysics` (`self.Head`) true)
      (`PrimitiveComponent.SetSimulatePhysics` (`self.Neck`) true)
      (`KismetSystemLibrary.Delay` 3.0)
      (`self.K2_DestroyActor`))))

(event `self.ReceiveBeginPlay`
  (bind _returnvalue (`|CreateWidget` "/Game/Blueprints/UI/MainHUD.MainHUD_C"))
  (`UserWidget.AddToViewport` _returnvalue 0))

(fn `UserConstructionScript`)